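; BP_TestTile is a test tile Blueprint whose construction script and NewFunction currently do nothing.
; Disconnected construction-script logic would spawn a static mesh component at the saved relative transform for each PropArray entry, and a preview mesh for each ObstacleArray entry.
; An empty loop over existing static mesh components is also left unwired, so none of this runs.
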(fn ConstructionScript)

(fn NewFunction)